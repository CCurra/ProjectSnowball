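; Generator interactable that responds when the player reaches it carrying a battery.
; On BeginPlay it stores the first Elevator actor found in the level as its target.
; When the player pawn overlaps its Box, it checks GotBattery on the ThirdPersonCharacter and, if true, destroys that Elevator actor.
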(event `self.Box.OnComponentBeginOverlap`
  (params (OverlappedComponent :type "PrimitiveComponent Object Reference") (OtherActor :type "Actor Object Reference") (OtherComp :type "PrimitiveComponent Object Reference") (OtherBodyIndex :type Integer) (bFromSweep :type Boolean) (SweepResult :type "HitResult Structure (by ref)"))
  ;[1 1 1] Player Collision
  (if (== OtherActor (`GameplayStatics.GetPlayerPawn` 0))
    (bind _asthird_person_character (cast `/Game/ThirdPersonBP/Blueprints/ThirdPersonCharacter` OtherActor))
    (if (`/Game/ThirdPersonBP/Blueprints/ThirdPersonCharacter.Got Battery` _asthird_person_character)
      (bind _asactor (cast `Actor` (`self.TargetElevator`)))
      (`self.K2_DestroyActor` _asactor))))

(event `self.ReceiveBeginPlay`
  ;[1 1 1] Sets Elevator
  (bind _outactors (`GameplayStatics.GetAllActorsOfClass` "/Game/Blueprints/Interactables/Elevator.Elevator_C"))
  (set `self.TargetElevator` (`|GetArrayItem` _outactors)))

(fn `UserConstructionScript`)