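; An overlap-triggered button that rotates the level's Platform180 actor.
; On BeginPlay it caches the first Platform180 found; when the player pawn enters its Box, it plays a timeline from the start.
; Each timeline update adds a fixed, swept local rotation to the platform's root, so the total turn depends on frame rate.
; A Start flag blocks retriggering until the timeline finishes.
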(event `self.ReceiveBeginPlay`
  (bind _outactors (`GameplayStatics.GetAllActorsOfClass` "/Game/ThirdPersonBP/Platform180.Platform180_C"))
  (set `self.Platform180` (`|GetArrayItem` _outactors)))

(event `self.Box.OnComponentBeginOverlap`
  (params (OverlappedComponent :type "PrimitiveComponent Object Reference") (OtherActor :type "Actor Object Reference") (OtherComp :type "PrimitiveComponent Object Reference") (OtherBodyIndex :type Integer) (bFromSweep :type Boolean) (SweepResult :type "HitResult Structure (by ref)"))
  (if (== OtherActor (`GameplayStatics.GetPlayerPawn` 0))
    (bind _asplatform_180 (cast `/Game/ThirdPersonBP/Platform180` (`self.Platform180`)))
    (if (not (`self.Start`))
      (set `self.Start` true)
      (`Timeline|Timeline_0` :!via `PlayFromStart`
        (:`Update`
          (`SceneComponent.K2_AddLocalRotation` (`Actor.RootComponent` _asplatform_180) (struct :`Roll` 0.5) true false))
        (:`Finished`
          (set `self.Start` false))))))

(fn `UserConstructionScript`)