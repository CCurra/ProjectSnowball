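; Button interactable that raises a door when the player pawn overlaps its Box, then lowers it again.
; At BeginPlay it takes the first Door actor found in the level as its target.
; Two timelines add a fixed local Z offset per update, separated by a delay, so travel depends on frame rate.
; An Activated flag blocks retriggering until the lowering finishes.
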(event `self.ReceiveBeginPlay`
  (bind _outactors (`GameplayStatics.GetAllActorsOfClass` "/Game/ThirdPersonBP/Door.Door_C"))
  (set `self.Door` (`|GetArrayItem` _outactors)))

(event `self.Box.OnComponentBeginOverlap`
  (params (OverlappedComponent :type "PrimitiveComponent Object Reference") (OtherActor :type "Actor Object Reference") (OtherComp :type "PrimitiveComponent Object Reference") (OtherBodyIndex :type Integer) (bFromSweep :type Boolean) (SweepResult :type "HitResult Structure (by ref)"))
  (if (== OtherActor (`GameplayStatics.GetPlayerPawn` 0))
    (bind _asdoor (cast `/Game/ThirdPersonBP/Door` (`self.Door`)))
    (if (not (`self.Activated`))
      (set `self.Activated` true)
      (`Timeline|Timeline_0` :!via `PlayFromStart`
        (:`Update`
          (`SceneComponent.K2_AddLocalOffset` (`Actor.RootComponent` _asdoor) (0.0 0.0 0.5) false false))
        (:`Finished`
          (`KismetSystemLibrary.Delay` 3.0)
          (`Timeline|Timeline_1` :!via `PlayFromStart`
            (:`Update`
              (`SceneComponent.K2_AddLocalOffset` (`Actor.RootComponent` _asdoor) (0.0 0.0 -0.5) false false))
            (:`Finished`
              (set `self.Activated` false))))))))

(fn `UserConstructionScript`)