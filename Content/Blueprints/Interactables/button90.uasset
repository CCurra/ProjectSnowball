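; Button that rotates the level's Platform90 when the player pawn overlaps its box trigger.
; BeginPlay caches the first Platform90 found in the world.
; On overlap, a timeline steps the platform mesh's local rotation by a fixed, swept amount each update, so speed depends on frame rate.
; It stops early if the platform's actor rotation matches a 90-degree target within a small tolerance.
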(event `self.ReceiveBeginPlay`
  (bind _outactors (`GameplayStatics.GetAllActorsOfClass` "/Game/Blueprints/Interactables/Platform90.Platform90_C"))
  (set `self.Platform90` (`|GetArrayItem` _outactors)))

(event `self.Box.OnComponentBeginOverlap`
  (params (OverlappedComponent :type "PrimitiveComponent Object Reference") (OtherActor :type "Actor Object Reference") (OtherComp :type "PrimitiveComponent Object Reference") (OtherBodyIndex :type Integer) (bFromSweep :type Boolean) (SweepResult :type "HitResult Structure (by ref)"))
  (if (== OtherActor (`GameplayStatics.GetPlayerPawn` 0))
    (set `self.Start` true)
    (bind _asplatform_90 (cast `/Game/Blueprints/Interactables/Platform90` (`self.Platform90`)))
    (`Timeline|Timeline_0` :!via `PlayFromStart` :!label _label
      (:`Update`
        (`|ExecutionSequence`
          (:`then_0`
            (`SceneComponent.K2_AddLocalRotation` (`StaticMeshActor.StaticMeshComponent` _asplatform_90) (struct :`Roll` -0.5) true false))
          (:`then_1`
            (if (== (`self.K2_GetActorRotation` _asplatform_90) (struct :`Roll` 90.0))
              (goto _label :!via `Stop`))))))))

(fn `UserConstructionScript`)